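; NormalMagicEffect is a magic effect actor that applies a radial force when something overlaps it.
; Each tick it scales the RadialForce impulse and force strength from the particle system's world X scale.
; The first overlap activates the force and sets a short life span so the actor soon destroys itself.
; A Spawn event stores an attack value, which this graph does not otherwise use.
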(event `self.ReceiveTick`
  (params (DeltaSeconds :type "Float (single-precision)"))
  (bind _radialforce (`self.RadialForce`))
  (bind _returnvalue_x (`KismetMathLibrary.BreakVector` (`SceneComponent.K2_GetComponentScale` (`self.ParticleSystem`))))
  (bind _output_get (set `RadialForceComponent.ImpulseStrength` (* 10000 _returnvalue_x) _radialforce))
  (set `RadialForceComponent.ForceStrength` _output_get _radialforce))

(event `Spawn`
  (params (atk :type Integer))
  (set `self.atk` atk))

(event `self.ReceiveActorBeginOverlap`
  (params (OtherActor :type "Actor Object Reference"))
  (`ActorComponent.Activate` (`self.RadialForce`) false)
  (`self.SetLifeSpan` 0.3))

(fn `UserConstructionScript`)
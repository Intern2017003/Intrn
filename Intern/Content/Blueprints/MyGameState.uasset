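; Game state Blueprint that tracks a combo count and a score-derived Rate value.
; A looping 15-second delay started on BeginPlay compares Combo to its last snapshot, resets it to zero if it has not grown, then stores a new snapshot.
; Tick continuously recalculates Rate as Score divided by a fixed constant.
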(event `self.ReceiveBeginPlay`
  (`KismetSystemLibrary.Delay` 15.0 :!label _label)
  (if (not (> (`self.Combo`) (`self.Tcombo`)))
    (set `self.Combo` 0))
  (set `self.Tcombo` (`self.Combo`))
  (goto _label))

(event `self.ReceiveTick`
  (params (DeltaSeconds :type "Float (single-precision)"))
  (set `self.Rate` (/ (`KismetMathLibrary.Conv_IntToDouble` (`self.Score`)) 5000.0)))

(fn `UserConstructionScript`)
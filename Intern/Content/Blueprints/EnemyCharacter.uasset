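; Enemy character Blueprint that takes damage from magic projectiles and hurts the player on contact.
; Overlapping a NormalMagicEffect subtracts its Atk from HP after a short delay, gated by a one-second DoOnce cooldown.
; At zero HP it spawns an impact emitter, expires via a near-zero lifespan and adds EScore to the MyGameState score once.
; ATKCollision overlaps subtract EATK from the ThirdPersonCharacter's LifePoint, also rate-limited to once per second.
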(event `self.ReceiveActorBeginOverlap`
  (params (OtherActor :type "Actor Object Reference"))
  ;[1 1 1] EnemyHP
  (bind _asnormal_magic_effect (cast `/Game/Blueprints/NormalMagicEffect` OtherActor))
  (`/Engine/EditorBlueprintResources/StandardMacros.DoOnce` false :!label _label
    (:`Completed`
      (`|ExecutionSequence`
        (:`then_0`
          (`KismetSystemLibrary.Delay` 1.0)
          (goto _label :!via `Reset`))
        (:`then_1`
          (`KismetSystemLibrary.Delay` 0.1)
          (bind _output_get (set `self.HP` (- (`self.HP`) (`/Game/Blueprints/NormalMagicEffect.atk` _asnormal_magic_effect))))
          (`KismetSystemLibrary.PrintString` (`KismetStringLibrary.Conv_IntToString` _output_get))
          (if (<= _output_get 0)
            ;[1 1 1] Dead
            (`GameplayStatics.SpawnEmitterAtLocation` "/Game/InfinityBladeEffects/Effects/FX_Monsters/FX_Monster_Ausar/P_AU_Trap_Impact.P_AU_Trap_Impact" (`self.K2_GetActorLocation`))
            (`self.SetLifeSpan` 1e-06)
            (`/Engine/EditorBlueprintResources/StandardMacros.DoOnce` false
              (:`Completed`
                (bind _asmy_game_state (cast `/Game/Blueprints/MyGameState` (`GameplayStatics.GetGameState`)))
                (set `/Game/Blueprints/MyGameState.Score` (+ (`/Game/Blueprints/MyGameState.Score` _asmy_game_state) (`self.EScore`)) _asmy_game_state)))))))))

(event `self.ATKCollision.OnComponentBeginOverlap`
  (params (OverlappedComponent :type "PrimitiveComponent Object Reference") (OtherActor :type "Actor Object Reference") (OtherComp :type "PrimitiveComponent Object Reference") (OtherBodyIndex :type Integer) (bFromSweep :type Boolean) (SweepResult :type "HitResult Structure (by ref)"))
  ;[1 1 1] ATk
  (bind _asthird_person_character (cast `/Game/Blueprints/ThirdPersonCharacter` OtherActor))
  (`/Engine/EditorBlueprintResources/StandardMacros.DoOnce` false :!label _label_2
    (:`Completed`
      (set `/Game/Blueprints/ThirdPersonCharacter.LifePoint` (- (`/Game/Blueprints/ThirdPersonCharacter.LifePoint` _asthird_person_character) (`self.EATK`)) _asthird_person_character)
      (`KismetSystemLibrary.Delay` 1.0)
      (goto _label_2 :!via `Reset`))))

(fn `UserConstructionScript`)
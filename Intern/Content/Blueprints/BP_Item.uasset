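; BP_Item is a healing pickup that restores life to the ThirdPersonCharacter that overlaps it.
; On overlap it spawns a heal particle at its own location, adds RecoveryAmount to the character's LifePoint, and attaches a potion effect to the character's mesh.
; It then sets a short lifespan so the item destroys itself shortly after pickup, with no clamp on the life total.
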(event `self.ReceiveActorBeginOverlap`
  (params (OtherActor :type "Actor Object Reference"))
  (bind _asthird_person_character (cast `/Game/Blueprints/ThirdPersonCharacter` OtherActor))
  (`GameplayStatics.SpawnEmitterAtLocation` "/Game/InfinityBladeEffects/Effects/FX_Ability/Heal/P_Heal_LongDistance_Start.P_Heal_LongDistance_Start" (`self.K2_GetActorLocation`))
  (set `/Game/Blueprints/ThirdPersonCharacter.LifePoint` (+ (`/Game/Blueprints/ThirdPersonCharacter.LifePoint` _asthird_person_character) (`self.RecoveryAmount`)) _asthird_person_character)
  (`GameplayStatics.SpawnEmitterAttached` "/Game/InfinityBladeEffects/Effects/FX_Ability/Heal/P_Heal_Potion.P_Heal_Potion" (`Character.Mesh` _asthird_person_character) "None" (`self.K2_GetActorLocation` _asthird_person_character) (struct) "KeepWorldPosition")
  (`self.SetLifeSpan` 0.2))

(fn `UserConstructionScript`)
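; NormalMagic is a magic projectile actor that can be charged and detonates into a NormalMagicEffect.
; ChargeLevel scales the projectile by the charge value and multiplies its base attack by it to set ATK.
; Detonation, called directly or triggered by hitting anything not tagged Safe, spawns the effect at the actor's location, scaled by charge, and passes it ATK.
; It then calls SetLifeSpan with zero.
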(event `Detonated`
  (bind _returnvalue (`|SpawnActorFromClass` "/Game/Blueprints/NormalMagicEffect.NormalMagicEffect_C" (`KismetMathLibrary.MakeTransform` (`self.K2_GetActorLocation`) (struct) (* (1.0 1.0 1.0) (stale `ChargeLevel` B))) "Undefined" "OverrideRootScale" :!label _label))
  (`/Game/Blueprints/NormalMagicEffect.Spawn` _returnvalue (`self.ATK`))
  (`self.SetLifeSpan` 1e-07))

(event `self.ReceiveHit`
  (params (MyComp :type "PrimitiveComponent Object Reference") (Other :type "Actor Object Reference") (OtherComp :type "PrimitiveComponent Object Reference") (bSelfMoved :type Boolean) (HitLocation :type "Vector Structure") (HitNormal :type "Vector Structure") (NormalImpulse :type "Vector Structure") (Hit :type "HitResult Structure (by ref)"))
  (if (not (`self.ActorHasTag` Other "Safe"))
    (goto _label)))

(event `ChargeLevel`
  (params (B :type "Float (double-precision)"))
  (`self.SetActorScale3D` (* (0.1 0.1 0.1) B))
  (set `self.ATK` (`KismetMathLibrary.FTrunc` (* (`self.ATK_base`) B))))

(fn `UserConstructionScript`)
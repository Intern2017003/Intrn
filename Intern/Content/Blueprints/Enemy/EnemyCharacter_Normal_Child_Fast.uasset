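; A fast enemy character variant, named FLASH, that leaves a poison charge particle trail as it moves.
; BeginPlay runs the parent logic, then overrides health, attack, score and name.
; Tick checks for nonzero velocity and, after a short Delay that throttles spawning, spawns the trail emitter at the capsule's location with the actor's rotation.
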(event `self.ReceiveBeginPlay`
  (`parent.ReceiveBeginPlay`)
  (set `self.HP` 1000)
  (set `self.HP_MAX` 1000)
  (set `self.EATK` 200)
  (set `self.EScore` 50)
  (set `self.Name` "FLASH"))

(event `self.ReceiveTick`
  (params (DeltaSeconds :type "Float (single-precision)"))
  ;[1 1 1] Emitter
  (if (> (`KismetMathLibrary.VSize` (`self.GetVelocity`)) 0.0)
    (`KismetSystemLibrary.Delay` 0.03)
    (`GameplayStatics.SpawnEmitterAtLocation` "/Game/InfinityBladeEffects/Effects/FX_Monsters/FX_Monster_Wolf/Poison/P_ChargeTrail_Poison.P_ChargeTrail_Poison" (`SceneComponent.K2_GetComponentLocation` (`self.CapsuleComponent`)) (`self.K2_GetActorRotation`))))

(fn `UserConstructionScript`
  (`parent.UserConstructionScript`))
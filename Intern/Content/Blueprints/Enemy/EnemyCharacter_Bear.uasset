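; Bear boss enemy character that takes magic hits, attacks the player, and opens the Clear level on death.
; Once unlocked, NormalMagicEffect overlaps apply rate-scaled, throttled damage, publish boss stats to MyGameState and drive AnimBP reactions, with death awarding score and combo.
; Aim overlap opens a Tick-fed gate for repeated facing and attacking.
; ATKCollision overlaps open and close gates controlling delayed player damage, with DoOnce resets as cooldowns.
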(event `self.ReceiveBeginPlay`
  (set `self.HP` (`self.HP_MAX`))
  (bind _asbear_anim_bp (cast `/Game/Blueprints/Enemy/Bear_AnimBP` (`SkeletalMeshComponent.GetAnimInstance` (`self.Mesh`))))
  (set `self.AnimBP` _asbear_anim_bp))

(event `self.ReceiveActorBeginOverlap`
  (params (OtherActor :type "Actor Object Reference"))
  ;[1 1 1] EnemyHP
  (`/Engine/EditorBlueprintResources/StandardMacros.Gate` false :!label _label
    (:`Exit`
      (bind _asnormal_magic_effect (cast `/Game/Blueprints/NormalMagicEffect` OtherActor))
      (`/Engine/EditorBlueprintResources/StandardMacros.DoOnce` false :!label _label_2
        (:`Completed`
          (`|ExecutionSequence`
            (:`then_0`
              (`KismetSystemLibrary.Delay` 1.0)
              (goto _label_2 :!via `Reset`))
            (:`then_1`
              (`KismetSystemLibrary.Delay` 0.1)
              (bind _output_get (set `self.HP` (- (`self.HP`) (`KismetMathLibrary.FTrunc` (* (`/Game/Blueprints/NormalMagicEffect.atk` _asnormal_magic_effect) (`self.DamegeRate`))))))
              (bind _asmy_game_state (cast `/Game/Blueprints/MyGameState` (`GameplayStatics.GetGameState`)))
              (bind _output_get_2 (set `/Game/Blueprints/MyGameState.BOSSHP` (`self.HP`) _asmy_game_state))
              (set `/Game/Blueprints/MyGameState.EHP` _output_get_2 _asmy_game_state)
              (bind _output_get_3 (set `/Game/Blueprints/MyGameState.BOSSHPM` (`self.HP_MAX`) _asmy_game_state))
              (set `/Game/Blueprints/MyGameState.EHPM` _output_get_3 _asmy_game_state)
              (set `/Game/Blueprints/MyGameState.NAME` (`self.Name`) _asmy_game_state)
              (if (<= _output_get 0)
                ;[1 1 1] Dead
                (`/Game/Blueprints/Enemy/Bear_AnimBP.Die` (`self.AnimBP`))
                (`/Engine/EditorBlueprintResources/StandardMacros.DoOnce` false
                  (:`Completed`
                    (set `/Game/Blueprints/MyGameState.Score` (+ (`/Game/Blueprints/MyGameState.Score` _asmy_game_state) (`self.EScore`)) _asmy_game_state)
                    (`/Engine/EditorBlueprintResources/StandardMacros.IncrementInt` (`/Game/Blueprints/MyGameState.Combo` _asmy_game_state)
                      (:`  `
                        (bind _asmy_game_instance (cast `/Game/Blueprints/MyGameInstance` (`GameplayStatics.GetGameInstance`)))
                        (`/Game/Blueprints/MyGameInstance.Global` _asmy_game_instance)
                        (`GameplayStatics.OpenLevel` "Clear")))))
                (else
                  (set `self.DamegeRate` (`/Game/Blueprints/MyGameState.Rate` _asmy_game_state)))))
            (:`then_2`
              (`/Game/Blueprints/Enemy/Bear_AnimBP.Damage` (`self.AnimBP`)))))))))

(event `Unlock`
  ;[1 1 1] EnemyHP
  (goto _label :!via `Open`))

(event `self.ReceiveTick`
  (params (DeltaSeconds :type "Float (single-precision)"))
  (bind (_returnvalue_roll _returnvalue_pitch _returnvalue_yaw) (`KismetMathLibrary.BreakRotator` (`KismetMathLibrary.FindLookAtRotation` (`self.K2_GetActorLocation`) (`self.K2_GetActorLocation` (`GameplayStatics.GetPlayerCharacter` 0)))))
  ;[1 1 1] ATk
  (`/Engine/EditorBlueprintResources/StandardMacros.Gate` true :!label _label_3
    (:`Exit`
      (`|ExecutionSequence`
        (:`then_0`
          (`/Engine/EditorBlueprintResources/StandardMacros.DoOnce` false :!label _label_4
            (:`Completed`
              (`/Game/Blueprints/Enemy/Bear_AnimBP.Attack!` (`self.AnimBP`) :!label _label_5)
              (`KismetSystemLibrary.Delay` 1.5)
              (`/Engine/EditorBlueprintResources/StandardMacros.Gate` true :!label _label_6
                (:`Exit`
                  (`/Engine/EditorBlueprintResources/StandardMacros.DoOnce` false :!label _label_7
                    (:`Completed`
                      (bind _asthird_person_character (cast `/Game/Blueprints/ThirdPersonCharacter` (`GameplayStatics.GetPlayerCharacter` 0)))
                      (`/Game/Blueprints/ThirdPersonCharacter.Damage` _asthird_person_character (`self.EATK`))
                      (`KismetSystemLibrary.Delay` 1.0)
                      (goto _label_7 :!via `Reset`))))))))
        (:`then_1`
          (goto _label_6 :!via `Open`))
        (:`then_2`
          (goto _label_5))
        (:`then_3`
          (`MovementComponent.StopMovementImmediately` (`self.CharacterMovement`))
          (`self.K2_SetActorRotation` (`KismetMathLibrary.MakeRotator` 0.0 0.0 _returnvalue_yaw)))
        (:`then_4`
          (`KismetSystemLibrary.Delay` 3.0)
          (goto _label_4 :!via `Reset`))))))

(event `self.Aim.OnComponentBeginOverlap`
  (params (OverlappedComponent :type "PrimitiveComponent Object Reference") (OtherActor :type "Actor Object Reference") (OtherComp :type "PrimitiveComponent Object Reference") (OtherBodyIndex :type Integer) (bFromSweep :type Boolean) (SweepResult :type "HitResult Structure (by ref)"))
  ;[1 1 1] ATk
  (cast `/Game/Blueprints/ThirdPersonCharacter` OtherActor)
  (goto _label_3 :!via `Open`))

(event `self.ATKCollision.OnComponentEndOverlap`
  (params (OverlappedComponent :type "PrimitiveComponent Object Reference") (OtherActor :type "Actor Object Reference") (OtherComp :type "PrimitiveComponent Object Reference") (OtherBodyIndex :type Integer))
  ;[1 1 1] ATk
  (cast `/Game/Blueprints/ThirdPersonCharacter` OtherActor)
  (`|ExecutionSequence`
    (:`then_0`
      (goto _label_3 :!via `Close`))
    (:`then_1`
      (goto _label_6 :!via `Close`))))

(event `self.ATKCollision.OnComponentBeginOverlap`
  (params (OverlappedComponent :type "PrimitiveComponent Object Reference") (OtherActor :type "Actor Object Reference") (OtherComp :type "PrimitiveComponent Object Reference") (OtherBodyIndex :type Integer) (bFromSweep :type Boolean) (SweepResult :type "HitResult Structure (by ref)"))
  ;[1 1 1] ATk
  (cast `/Game/Blueprints/ThirdPersonCharacter` OtherActor)
  (goto _label_6 :!via `Open`))

(fn `UserConstructionScript`)
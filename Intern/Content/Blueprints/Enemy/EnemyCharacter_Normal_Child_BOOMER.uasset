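; BOOMER enemy character, a child Blueprint that explodes when the player touches its attack collision or when its HP runs out.
; Overlapping magic effects subtract their attack value from HP, gated by a one-second DoOnce reset, and publish HP and name to MyGameState.
; Death adds score and combo once, then calls Boom, which spawns EnemyExplotion and expires the actor shortly after; contact detonation skips the reward.
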(event `self.ReceiveBeginPlay`
  (`parent.ReceiveBeginPlay`)
  (set `self.HP` 5000)
  (set `self.HP_MAX` 5000)
  (set `self.EATK` 0)
  (set `self.EScore` 1000)
  (set `self.Name` "BOOMER"))

(event `self.ReceiveActorBeginOverlap`
  (params (OtherActor :type "Actor Object Reference"))
  ;[1 1 1] EnemyHP
  (bind _asnormal_magic_effect (cast `/Game/Blueprints/NormalMagicEffect` OtherActor))
  (`/Engine/EditorBlueprintResources/StandardMacros.DoOnce` false :!label _label
    (:`Completed`
      (`|ExecutionSequence`
        (:`then_0`
          (`KismetSystemLibrary.Delay` 1.0)
          (goto _label :!via `Reset`))
        (:`then_1`
          (`KismetSystemLibrary.Delay` 0.1)
          (bind _output_get (set `self.HP` (- (`self.HP`) (`/Game/Blueprints/NormalMagicEffect.atk` _asnormal_magic_effect))))
          (bind _asmy_game_state (cast `/Game/Blueprints/MyGameState` (`GameplayStatics.GetGameState`)))
          (set `/Game/Blueprints/MyGameState.EHP` (`self.HP`) _asmy_game_state)
          (set `/Game/Blueprints/MyGameState.EHPM` (`self.HP_MAX`) _asmy_game_state)
          (set `/Game/Blueprints/MyGameState.NAME` (`self.Name`) _asmy_game_state)
          (if (<= _output_get 0)
            ;[1 1 1] Dead
            (`/Engine/EditorBlueprintResources/StandardMacros.DoOnce` false
              (:`Completed`
                (bind _asmy_game_state_2 (cast `/Game/Blueprints/MyGameState` (`GameplayStatics.GetGameState`)))
                (set `/Game/Blueprints/MyGameState.Score` (+ (`/Game/Blueprints/MyGameState.Score` _asmy_game_state_2) (`self.EScore`)) _asmy_game_state_2)
                (`/Engine/EditorBlueprintResources/StandardMacros.IncrementInt` (`/Game/Blueprints/MyGameState.Combo` _asmy_game_state_2)
                  (:`  `
                    (`self.boom`)))))))))))

(event `boom`
  ;[1 1 1] ATk
  (`|SpawnActorFromClass` "/Game/Blueprints/Enemy/EnemyExplotion.EnemyExplotion_C" (`KismetMathLibrary.MakeTransform` (`self.K2_GetActorLocation`)) "Undefined" "OverrideRootScale" :!label _label_2)
  (`self.SetLifeSpan` 0.2))

(event `self.ATKCollision.OnComponentBeginOverlap`
  (params (OverlappedComponent :type "PrimitiveComponent Object Reference") (OtherActor :type "Actor Object Reference") (OtherComp :type "PrimitiveComponent Object Reference") (OtherBodyIndex :type Integer) (bFromSweep :type Boolean) (SweepResult :type "HitResult Structure (by ref)"))
  ;[1 1 1] ATk
  (cast `/Game/Blueprints/ThirdPersonCharacter` OtherActor)
  (goto _label_2))

(fn `UserConstructionScript`
  (`parent.UserConstructionScript`))